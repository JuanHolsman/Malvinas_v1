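; Sheep character Blueprint that wanders on its own and flees when the third-person player touches it.
; A decision loop, gated by CanMove, waits a random 1–3 seconds, then roams slowly to a nearby reachable point via AIMoveTo.
; Capsule overlap with the player calls RunAway directly, sprinting to a random, non-directional point in a much larger radius.
; Only successful moves restart the loop, and ShouldRun is never set true here.
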(event `self.ReceiveBeginPlay`
  (if (`self.CanMove?`)
    (`self.DecideNextAction` false)))

(event `DecideNextAction`
  (params (`SkipDelay?` :type Boolean))
  ;[1 1 1] Decide Action
  (if (`self.CanMove?`)
    (if (not `SkipDelay?`)
      (`KismetSystemLibrary.Delay` (`KismetMathLibrary.Conv_IntToDouble` (`KismetMathLibrary.RandomIntegerInRange` 1 3))))
    (if (`self.ShouldRun?`)
      (`self.RunAway`)
      (else
        (`self.RandomRoam`)))))

(event `RandomRoam`
  ;[1 1 1] Random Roam
  (if (`self.CanMove?`)
    (set `CharacterMovementComponent.MaxWalkSpeed` 150.0 (`self.CharacterMovement`))
    (if (`self.CanMove?`)
      (`|AIMoveTo` self (`NavigationSystemV1.K2_GetRandomReachablePointInRadius` (`self.K2_GetActorLocation`) 1500.0 null null) null
        (:`OnSuccess`
          (`self.DecideNextAction` false))))))

(event `RunAway`
  ;[1 1 1] Run Away
  (if (`self.CanMove?`)
    (set `CharacterMovementComponent.MaxWalkSpeed` 600.0 (`self.CharacterMovement`))
    (if (`self.CanMove?`)
      (`|AIMoveTo` self (`NavigationSystemV1.K2_GetRandomReachablePointInRadius` (`self.K2_GetActorLocation`) (`KismetMathLibrary.RandomFloatInRange` 20000.0 30000.0) null null) null
        (:`OnSuccess`
          (set `self.ShouldRun?` false)
          (`self.DecideNextAction` true))))))

(event `self.CapsuleComponent.OnComponentBeginOverlap`
  (params (OverlappedComponent :type "PrimitiveComponent Object Reference") (OtherActor :type "Actor Object Reference") (OtherComp :type "PrimitiveComponent Object Reference") (OtherBodyIndex :type Integer) (bFromSweep :type Boolean) (SweepResult :type "HitResult Structure (by ref)"))
  (if (`self.CanMove?`)
    (cast `/Game/ThirdPersonBP/Blueprints/ThirdPersonCharacter` OtherActor)
    (if (`self.CanMove?`)
      (`self.RunAway`)
      (`KismetSystemLibrary.PrintString` "Hello"))))

(fn `UserConstructionScript`)