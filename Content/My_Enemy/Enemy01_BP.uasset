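; Enemy pawn Blueprint that patrols a set of points and chases actors tagged Player.
; On BeginPlay it sets a walk speed and loops through PatrolPoints with AI MoveTo, advancing and wrapping PointIndex on each success.
; Any AIPerception target update raises the walk speed, then moves toward the actor if tagged Player, repeating on success.
; The perception stimulus is not checked, and nothing restores patrol speed or explicitly restarts patrolling.
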(event `Chase Player`
  ;[1 1 1] Atrapar Jugador
  (set `CharacterMovementComponent.MaxWalkSpeed` 600.0 (`self.CharacterMovement`) :!label _label)
  (if (`self.ActorHasTag` (stale `self.AIPerception.OnTargetPerceptionUpdated` Actor) "Player")
    (`|AIMoveTo` self (0.0 0.0 0.0) (stale `self.AIPerception.OnTargetPerceptionUpdated` Actor) 50.0
      (:`OnSuccess`
        (`self.Chase Player`)))))

(event `self.AIPerception.OnTargetPerceptionUpdated`
  (params (Actor :type "Actor Object Reference") (Stimulus :type "AIStimulus Structure"))
  ;[1 1 1] Atrapar Jugador
  (goto _label))

(event `self.ReceiveBeginPlay`
  ;[1 1 1] Patrullaje
  (set `CharacterMovementComponent.MaxWalkSpeed` 300.0 (`self.CharacterMovement`))
  (`self.Patrol To Point`))

(event `Patrol To Point`
  ;[1 1 1] Patrullaje
  (`|AIMoveTo` self (0.0 0.0 0.0) (`|GetArrayItem` (`self.PatrolPoints`) (`self.PointIndex`))
    (:`OnSuccess`
      (if (>= (`self.PointIndex`) (- (`KismetArrayLibrary.Array_Length` (`self.PatrolPoints`)) 1))
        (set `self.PointIndex` 0)
        (else
          (`/Engine/EditorBlueprintResources/StandardMacros.IncrementInt` (`self.PointIndex`)
            (:`  `
              _))))
      (`self.Patrol To Point`))))

(fn `UserConstructionScript`)