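; Trigger actor with a missile that announces when the third-person character enters its area and can explode to kill that character.
; Overlap stores the character and fires the EventoBuscarNotas dispatcher.
; Explotar, not called within this Blueprint, hides the missile, spawns explosion effects, sound and camera shake, then zeroes the stored character's Health after a delay.
; That delay reads the emitter's CustomTimeDilation as its duration, while a TiempoExplote delay is left unconnected.
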(event `self.TriggerArea.OnComponentBeginOverlap`
  (params (OverlappedComponent :type "PrimitiveComponent Object Reference") (OtherActor :type "Actor Object Reference") (OtherComp :type "PrimitiveComponent Object Reference") (OtherBodyIndex :type Integer) (bFromSweep :type Boolean) (SweepResult :type "HitResult Structure (by ref)"))
  (bind _asthird_person_character (cast `/Game/ThirdPersonBP/Blueprints/ThirdPersonCharacter` OtherActor))
  (`self.EventoBuscarNotas`))

(event `Explotar`
  (bind _returnvalue (`SceneComponent.K2_GetComponentLocation` (`self.misil`)))
  (`SceneComponent.SetVisibility` (`self.misil`) false true)
  (`GameplayStatics.SpawnEmitterAtLocation` "/Game/InfinityBladeEffects/Effects/FX_Monsters/FX_Monster_Gruntling/FlameThrower/P_FlameExplode.P_FlameExplode" _returnvalue (struct) (3.0 3.0 3.0))
  (bind _returnvalue_2 (`GameplayStatics.SpawnEmitterAtLocation` "/Game/InfinityBladeEffects/Effects/FX_Mobile/combat/P_ProjectileLob_Explo_Untyped.P_ProjectileLob_Explo_Untyped" _returnvalue (struct) (3.0 3.0 3.0)))
  (`GameplayStatics.SpawnSoundAttached` "/Game/StarterContent/Audio/Explosion01.Explosion01" _returnvalue_2 "None" (0.0 0.0 0.0) (struct) "KeepRelativeOffset" false 1.0 1.0 0.0 null null)
  (`GameplayStatics.PlayWorldCameraShake` "/Game/Shake2.Shake2_C" _returnvalue 0.0 100000.0)
  (`KismetSystemLibrary.Delay` (`ParticleSystemComponent.CustomTimeDilation` _returnvalue_2))
  (set `/Game/ThirdPersonBP/Blueprints/ThirdPersonCharacter.Health` 0.0 (stale `self.TriggerArea.OnComponentBeginOverlap` _asthird_person_character)))

(event `self.TriggerArea.OnComponentEndOverlap`
  (params (OverlappedComponent :type "PrimitiveComponent Object Reference") (OtherActor :type "Actor Object Reference") (OtherComp :type "PrimitiveComponent Object Reference") (OtherBodyIndex :type Integer)))

(fn `UserConstructionScript`)